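; Base interactive actor that can be activated once every interactive in its UnlockInteract list is active, or freely if that list is empty.
; Interact sets IsActivate and, if DelayBeforeDesactivate is set, switches it off after that delay.
; A widget tints green when active, yellow when available and red when locked.
; When ShowIntertactUI is enabled, sphere overlaps toggle the widget only for the player-controlled entity's capsule.
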(event OnComponentBeginOverlap(SphereCollision)
  (params (OverlappedComponent :type Primitive%20Component%20Object%20Reference) (OtherActor :type Actor%20Object%20Reference) (OtherComp :type Primitive%20Component%20Object%20Reference) (OtherBodyIndex :type Integer) (bFromSweep :type Boolean) (SweepResult :type Hit%20Result%20Structure%20%28by%20ref%29))
  (Utilities|FlowControl|Sequence
    (:then_0
      (if (Variables|Default|GetShowIntertactUI)
        ;[1 1 1] Show Widget only when player pass
        (bind _asbp_controllable_entity (Utilities|Casting|CastToBP_ControllableEntity OtherActor))
        (if (and (== (Variables|/Script/Engine.Character|GetCapsuleComponent _asbp_controllable_entity) OtherComp) (== (Utilities|GetClass (Game|GetInstigatorController OtherActor)) "/Game/Blueprint/BP_PlayerController.BP_PlayerController_C"))
          (Rendering|SetVisibility (Variables|Default|GetWidget) true false))))
    (:then_1
      (CallFunction|SetColorUI))))

(event OnComponentEndOverlap(SphereCollision)
  (params (OverlappedComponent :type Primitive%20Component%20Object%20Reference) (OtherActor :type Actor%20Object%20Reference) (OtherComp :type Primitive%20Component%20Object%20Reference) (OtherBodyIndex :type Integer))
  (if (Variables|Default|GetShowIntertactUI)
    ;[1 1 1] Remove widget only when player leave
    (bind _asbp_controllable_entity (Utilities|Casting|CastToBP_ControllableEntity OtherActor))
    (if (and (== (Variables|/Script/Engine.Character|GetCapsuleComponent _asbp_controllable_entity) OtherComp) (== (Utilities|GetClass (Game|GetInstigatorController OtherActor)) "/Game/Blueprint/BP_PlayerController.BP_PlayerController_C"))
      (Rendering|SetVisibility (Variables|Default|GetWidget) false false))))

(event Custom|Interact
  ;[1 1 1] Interact
  (if (Utilities|Array|IsEmpty (Variables|Default|GetUnlockInteract))
    (Variables|Default|SetisActivate? true)
    (Utilities|FlowControl|Sequence
      (:then_0
        (if (Variables|Default|GetdelayBeforeDesactivate?)
          (Utilities|FlowControl|Delay (Variables|Default|GetdelayBeforeDesactivate) :!label _label)
          (Variables|Default|SetisActivate? false)
          (CallFunction|SetColorUI)))
      (:then_1
        (CallFunction|SetColorUI)))
    (else
      (bind _bool (CallFunction|AllInteractUnlock?))
      (if _bool
        (Variables|Default|SetisActivate? true)
        (Utilities|FlowControl|Sequence
          (:then_0
            (if (Variables|Default|GetdelayBeforeDesactivate?)
              (goto _label)))
          (:then_1
            (CallFunction|SetColorUI)))))))

(event Custom|SetColorUI
  (bind _wbp_interact (Variables|Default|GetWBP_Interact))
  (if (Variables|Default|GetisActivate?)
    (Appearance|SetColorandOpacity (Variables|Default|GetWBP_Interact) "(R=0.204724,G=0.578125,B=0.162947,A=1.000000)" :!class /Script/UMG.UserWidget)
    (elif (Utilities|Array|IsEmpty (Variables|Default|GetUnlockInteract))
      (Appearance|SetColorandOpacity _wbp_interact "(R=0.578125,G=0.515829,B=0.084273,A=1.000000)" :!class /Script/UMG.UserWidget :!label _label)
      (else
        (bind _bool (CallFunction|AllInteractUnlock?))
        (if _bool
          (goto _label)
          (else
            (Appearance|SetColorandOpacity _wbp_interact "(R=0.578125,G=0.069984,B=0.000000,A=1.000000)" :!class /Script/UMG.UserWidget)))))))

(event EventBeginPlay
  (bind _aswbp_interact (Utilities|Casting|CastToWBP_Interact (UserInterface|GetUserWidgetObject (Variables|Default|GetWidget))))
  (Variables|Default|SetWBP_Interact _aswbp_interact)
  (CallFunction|SetColorUI))

(fn ConstructionScript)

(fn AllInteractUnlock?
  (bind _unlockedobject (LocalVariables|GetUnlockedObject))
  (bind _unlockinteract (Variables|Default|GetUnlockInteract))
  (if (not (Utilities|Array|IsEmpty _unlockinteract))
    (for _array_element _unlockinteract
      (Utilities|Array|Add _unlockedobject (Variables|BP_BaseInteractive_C|GetisActivate? _array_element)))
    (for _array_element_2 _unlockedobject
      (if (== _array_element_2 false)
        (return false)))
    (return true)))