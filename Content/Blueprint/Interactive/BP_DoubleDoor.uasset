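; BP_DoubleDoor is an interactive door that opens by disappearing and losing collision when activated.
; It extends a parent interactable's Interact, waits just past the activation delay, then hides the Door if IsActivate is set.
; Desactivation clears the flag, restores visibility and blocking collision, then calls the parent.
; BeginPlay runs the parent setup and sets the UI color.
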(event EventBeginPlay
  (|CallParentFunction)
  (CallFunction|SetUIColor))

(event EventInteract
  (params (DelayBeforeActivation :type Float%20%28double-precision%29))
  (|CallParentFunction DelayBeforeActivation)
  (Utilities|FlowControl|Delay (+ DelayBeforeActivation 0.01))
  (if (Variables|Default|GetisActivate?)
    (Rendering|SetVisibility (Variables|Default|GetDoor) false true)
    (Collision|SetCollisionProfileName (Variables|Default|GetDoor) "NoCollision" true :!class /Script/Engine.PrimitiveComponent)))

(fn ConstructionScript
  (|CallParentFunction))

(fn Desactivation
  (Variables|Default|SetisActivate? false)
  (Rendering|SetVisibility (Variables|Default|GetDoor) true true)
  (Collision|SetCollisionProfileName (Variables|Default|GetDoor) "BlockAllDynamic" true :!class /Script/Engine.PrimitiveComponent)
  (|CallParentFunction))