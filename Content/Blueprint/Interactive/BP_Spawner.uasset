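; Interactive spawner that periodically spawns monsters at its own location, up to a maximum number alive at once.
; From BeginPlay, a delay loop runs while IsActivate is false and ends for good once it finds the flag true.
; Each pass prunes invalid actors from ActorSpawned, then spawns MonsterToSpawn with its BehaviorTree and KillOnEndPossesse setting if below the cap.
; Interact only defers to the parent class.
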(event EventBeginPlay
  (|CallParentFunction)
  (Utilities|FlowControl|Delay 0.01)
  (if (not (Variables|Default|GetisActivate?)) :!label _label
    (bind _bool (CallFunction|MaxMonsterIsSpawned?))
    (if _bool
      _
      (else
        (bind _returnvalue (Game|SpawnActorfromClass (Variables|Default|GetMonsterToSpawn) (Math|Transform|MakeTransform (Transformation|GetActorLocation self) "0, 0, 0" "1.000000,1.000000,1.000000") "Undefined" 0 5e+01 6.0 1e+02 (Variables|Default|GetBehaviorTree) (Variables|Default|GetkillOnEndPossesse?) 0))
        (Utilities|Array|Add (Variables|Default|GetactorSpawned) _returnvalue)))
    (Utilities|FlowControl|Delay (Variables|Default|GetdelayBetweenEachSpawn))
    (goto _label)))

(event EventInteract
  (params (DelayBeforeActivation :type Float%20%28double-precision%29))
  (|CallParentFunction DelayBeforeActivation))

(fn ConstructionScript
  (|CallParentFunction))

(fn MaxMonsterIsSpawned?
  (bind _actorspawned (Variables|Default|GetactorSpawned))
  (for _array_element _actorspawned
    (Utilities|IsValid _array_element
      (:Is%20Not%20Valid
        (Utilities|Array|RemoveItem (Variables|Default|GetactorSpawned) _array_element))))
  (return (>= (Utilities|Array|Length _actorspawned) (Variables|Default|GetmaxMonsterToSpawn))))