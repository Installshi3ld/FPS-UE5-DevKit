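; BP_Button is an interactive button that switches itself on when interacted with.
; Interact runs the activation system, which activates immediately if UnlockInteract is empty, otherwise only when AllInteractUnlock passes.
; Activation updates the UI color and, when DelayBeforeDesactivate is set, switches the button off after that delay and refreshes the color again.
; BeginPlay calls the parent logic and sets the initial color.
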(event EventBeginPlay
  (|CallParentFunction)
  (CallFunction|SetUIColor))

(event EventInteract
  (|Activation/DesactivationSystem))

(fn ConstructionScript
  (|CallParentFunction))