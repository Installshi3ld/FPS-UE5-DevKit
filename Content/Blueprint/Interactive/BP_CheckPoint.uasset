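; BP_CheckPoint is an interactive checkpoint actor that records a checkpoint position for the player.
; Its Interact event runs the parent behavior, then casts player controller 0 to BP_PlayerController.
; It stores the Mesh's world location, raised along Z, in that controller's LastCheckpoint variable.
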(event EventBeginPlay
  (|CallParentFunction) ; This node is disabled and will not be called.\nDrag off pins to build functionality.
)

(event Collision|EventActorBeginOverlap
  (params (OtherActor :type Actor%20Object%20Reference)))

(event EventTick
  (params (DeltaSeconds :type Float%20%28single-precision%29)))

(event EventInteract
  (params (DelayBeforeActivation :type Float%20%28double-precision%29))
  (bind _mesh (Variables|Character|GetMesh))
  (bind _returnvalue (Transformation|GetWorldLocation _mesh))
  (|CallParentFunction DelayBeforeActivation)
  (bind _asbp_player_controller (Utilities|Casting|CastToBP_PlayerController (Game|GetPlayerController 0)))
  (Variables|/Game/Blueprint/BP_PlayerController.BP_PlayerController_C|SetLastCheckpoint _asbp_player_controller (Math|Vector|MakeVector (.x _returnvalue) (.y _returnvalue) (+ (.z _returnvalue) 2e+02))))

(fn ConstructionScript
  (|CallParentFunction))