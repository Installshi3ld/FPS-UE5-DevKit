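; Interactable weapon chest that spawns a set of weapons and lets the player take one per interaction.
; The first interaction spawns each DropWeapon class at SpawnLocation with evenly spaced yaw and zero scale.
; Later interactions map the overlapping character's yaw around the chest to an equal sector of the remaining stock.
; If that weapon's class enters the inventory, it becomes selected and the spawned actor is destroyed and unlisted.
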(event EventBeginPlay
  (|CallParentFunction) ; This node is disabled and will not be called.\nDrag off pins to build functionality.
)

(event Collision|EventActorBeginOverlap
  (params (OtherActor :type Actor%20Object%20Reference)))

(event EventTick
  (params (DeltaSeconds :type Float%20%28single-precision%29)))

(event EventInteract
  (params (DelayBeforeActivation :type Float%20%28double-precision%29))
  (bind _returnvalue (Transformation|GetActorLocation))
  (bind _stockedweapon (Variables|Default|GetStockedWeapon))
  (bind _spherecollision (Variables|Default|GetSphereCollision))
  (bind _stockedweapon_2 (Variables|Default|GetStockedWeapon))
  (bind _returnvalue_2 (Utilities|Array|Length _stockedweapon_2))
  (bind _overlappingactors (Collision|GetOverlappingActors _spherecollision "/Game/Blueprint/BP_MainCharacter.BP_MainCharacter_C" :!class /Script/Engine.PrimitiveComponent))
  (bind _output (Utilities|Array|Get(acopy) _overlappingactors))
  (bind _returnvalue_3 (/ 360 _returnvalue_2))
  (bind _returnvalue_4 (Transformation|GetActorLocation _output))
  (bind _returnvalue_5 (Math|Conversions|ToFloat(Integer) _returnvalue_3))
  (bind _returnvalue_6 (Math|Rotator|FindLookatRotation _returnvalue _returnvalue_4))
  (bind _returnvalue_7 (/ _returnvalue_5 2.0))
  (bind _returnvalue_8 (+ _returnvalue_7 (.yaw _returnvalue_6)))
  (bind _returnvalue_9 (< _returnvalue_8 0.0))
  (bind _returnvalue_10 (+ _returnvalue_8 3.6e+02))
  (bind _returnvalue_11 (Math|Float|SelectFloat _returnvalue_10 _returnvalue_8 _returnvalue_9))
  (bind _returnvalue_12 (/ _returnvalue_11 _returnvalue_5))
  (bind _returnvalue_13 (Math|Float|Floor _returnvalue_12))
  (bind _output_2 (Utilities|Array|Get(acopy) _stockedweapon _returnvalue_13))
  (if (Variables|Default|GetisActivate?)
    _
    (else
      (|CallParentFunction 0.0)))
  (if (Variables|Default|GetitemSpawned?)
    (bind _asbp_controllable_entity (Utilities|Casting|CastToBP_ControllableEntity (Utilities|Array|Get(acopy) (Collision|GetOverlappingActors (Variables|Default|GetSphereCollision) "/Game/Blueprint/BP_MainCharacter.BP_MainCharacter_C" :!class /Script/Engine.PrimitiveComponent))))
    (bind (_worked_ _indexininventory) (Default|AddWeapontoInventory _asbp_controllable_entity (Utilities|GetClass _output_2)))
    (if _worked_
      (Default|ChangeSelectedWeapon _asbp_controllable_entity _indexininventory)
      (Actor|DestroyActor _output_2)
      (Utilities|Array|RemoveItem (Variables|Default|GetStockedWeapon) _output_2))
    (else
      ;[1 1 1] CreateWeapon
      (for (_array_element _array_index) (Variables|Default|GetDropWeapon)
        (bind _returnvalue_14 (Game|SpawnActorfromClass _array_element (Math|Transform|MakeTransform (Transformation|GetWorldLocation (Variables|Default|GetSpawnLocation)) (Math|Rotator|MakeRotator 0.0 0.0 (Math|Conversions|ToFloat(Integer) (* (/ 360 (Utilities|Array|Length (Variables|Default|GetDropWeapon))) _array_index))) "0.000000,0.000000,0.000000") "Undefined" 0 0 0))
        (Utilities|Array|Add (Variables|Default|GetStockedWeapon) _returnvalue_14))
      (Variables|Default|SetitemSpawned? true))))

(fn ConstructionScript
  (|CallParentFunction))