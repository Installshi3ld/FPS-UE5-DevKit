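; Player character Blueprint that configures its movement and abilities from a data table on BeginPlay.
; A Sequence caches the "Player" row of DT_PlayerData, then applies walk speed, run speed, jump count, air control and the entity-change flag before calling the parent BeginPlay.
; ChangeVisibility and AddWeaponInInventory are empty, and leftover nodes that would attach a BP_AK child actor to the Arm never run.
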(event EventBeginPlay
  (Utilities|FlowControl|Sequence
    (:then_0
      (bind _returnvalue (Utilities|GetDataTableRow "/Game/Miscellaneous/DT_PlayerData.DT_PlayerData" "Player")
        (:then
          (Variables|Default|SetS_PlayerData _returnvalue))))
    (:then_1
      (bind _output_get (Variables|Default|SetbaseSpeed (.baseSpeed (Utilities|Struct|BreakS_Player (Variables|Default|GetS_PlayerData)))))
      (Variables|/Script/Engine.CharacterMovementComponent|SetMaxWalkSpeed (Variables|Character|GetCharacterMovement) _output_get)
      (Variables|Default|SetrunSpeed (.runSpeed (Utilities|Struct|BreakS_Player (Variables|Default|GetS_PlayerData))))
      (Variables|Default|SetJumpMaxCount (.jumpAmount (Utilities|Struct|BreakS_Player (Variables|Default|GetS_PlayerData))))
      (Variables|/Script/Engine.CharacterMovementComponent|SetAirControl (Variables|Character|GetCharacterMovement) (.airControl (Utilities|Struct|BreakS_Player (Variables|Default|GetS_PlayerData))))
      (Variables|Default|SetCanChangeEntity? (.canChangeEntity? (Utilities|Struct|BreakS_Player (Variables|Default|GetS_PlayerData))))
      (|CallParentFunction))))

(fn ConstructionScript
  (|CallParentFunction))

(fn ChangeVisibility)

(fn AddWeaponinInventory)