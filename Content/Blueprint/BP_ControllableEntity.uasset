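; Character that fights under AI or player control and can be taken over by the player while knocked.
; Knock damage fills a meter that flags the AI as knocked, then resets after a retriggerable delay.
; Pressing A possesses an overlapping knocked entity, whose meter drains as a possession timer before control reverts and AI resumes.
; Also handles movement, weapon inventory, interaction, ally/enemy tags and health with optional first-death protection.
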(event Custom|AddKnockValue
  (params (Value :type Float%20%28double-precision%29))
  (CallFunction|AddKnockValueFunc Value)
  (Utilities|ResetKnockValue false (Variables|KnockSystem|GetDelayBeforeUnknocked)))

(event Custom|OnPossesion
  (bind _returnvalue (Game|GetPlayerController 0))
  (bind _returnvalue_2 (Pawn|GetControlledPawn _returnvalue))
  (Utilities|StartDecreaseKnock)
  (if (== _returnvalue_2 self)
    (if (!= (Utilities|GetClass _returnvalue_2) "/Game/Blueprint/BP_MainCharacter.BP_MainCharacter_C")
      (bind _asbp_player_controller (Utilities|Casting|CastToBP_PlayerController (Game|GetPlayerController 0)))
      (Default|PossesSelf _asbp_player_controller)
      (Pawn|Possess (Variables|Default|GetAIController) self)
      (Default|ChangeKnockValue (Variables|Default|GetAIController) false))
    (else
      (Pawn|Possess (Variables|Default|GetAIController) self)
      (Default|ChangeKnockValue (Variables|Default|GetAIController) false))))

(event Game|Damage|EventAnyDamage
  (params (Damage :type Float%20%28single-precision%29) (DamageType :type Damage%20Type%20Object%20Reference) (InstigatedBy :type Controller%20Object%20Reference) (DamageCauser :type Actor%20Object%20Reference))
  ;[1 1 1] Damage system
  (if (not (Variables|HealthSystem|GetInvincible?))
    (bind _output_get (Variables|HealthSystem|Sethealth (- (Variables|HealthSystem|Gethealth) Damage)))
    (if (<= _output_get 0.0)
      (if (Variables|HealthSystem|GetavoidFirstDeath)
        (if (Variables|HealthSystem|GetavoidFirstDeathStatement)
          (Actor|DestroyActor self :!label _label)
          (else
            (Variables|HealthSystem|Sethealth 0.2)
            (Variables|HealthSystem|SetavoidFirstDeathStatement true)))
        (else
          (goto _label))))))

(event EventBeginPlay
  (bind _self self)
  (bind _tags (Variables|Actor|GetTags _self))
  (bind _asbp_base_weapon (Utilities|Casting|CastToBP_BaseWeapon (Variables|/Script/Engine.ChildActorComponent|GetChildActor (Variables|Default|GetWeapon))))
  (Utilities|Array|Add (Variables|WeaponInventory|GetWeaponInventory) _asbp_base_weapon)
  (Utilities|FlowControl|Sequence
    (:then_0
      (bind _astmp_debug_knock_value (Utilities|Casting|CastToTmp_DebugKnockValue (UserInterface|GetUserWidgetObject (Variables|Default|GetWidget))))
      (Variables|KnockSystem|SetKnockBar _astmp_debug_knock_value)
      (if (Variables|Default|GetisAlly)
        (Utilities|Array|AddUnique _tags "ally")
        (Utilities|Array|AddUnique (Variables|/Script/Engine.Actor|GetTags _asbp_base_weapon) "ally")
        (else
          (Utilities|Array|AddUnique _tags "enemy")
          (Utilities|Array|AddUnique (Variables|/Script/Engine.Actor|GetTags _asbp_base_weapon) "enemy"))))
    (:then_1
      (bind _asbp_base_ai_controller (Utilities|Casting|CastToBP_BaseAiController (AI|GetAIController self)))
      (Variables|Default|SetAIController _asbp_base_ai_controller))))

(event EventTick
  (params (DeltaSeconds :type Float%20%28single-precision%29))
  (bind _knockbar (Variables|KnockSystem|GetKnockBar))
  (Variables|/Game/Widget/Tmp_DebugKnockValue.Tmp_DebugKnockValue_C|SetknockBar _knockbar (Variables|KnockSystem|GetknockValue))
  (Variables|/Game/Widget/Tmp_DebugKnockValue.Tmp_DebugKnockValue_C|SetknockMax _knockbar (Variables|KnockSystem|GetknockValueMax)))

(event Input|ActionEvents|InputActionMouseButton1
  (params (Key :type Key%20Structure :default "None"))
  ;[1 1 1] Control
  (:Pressed
    (Default|ShootEvent (Utilities|Array|Get(acopy) (Variables|WeaponInventory|GetWeaponInventory) (Variables|WeaponInventory|GetCurrentEquipedWeapon)))))

(event Input|ActionEvents|InputActionJump
  (params (Key :type Key%20Structure :default "None"))
  ;[1 1 1] Control
  (:Pressed
    (Character|Jump)))

(event Input|ActionEvents|InputActionRun
  (params (Key :type Key%20Structure :default "None"))
  (bind _charactermovement (Variables|Character|GetCharacterMovement))
  ;[1 1 1] Control
  (:Pressed
    (Variables|/Script/Engine.CharacterMovementComponent|SetMaxWalkSpeed _charactermovement (Variables|Variable|GetrunSpeed)))
  (:Released
    (Variables|/Script/Engine.CharacterMovementComponent|SetMaxWalkSpeed _charactermovement (Variables|Variable|GetbaseSpeed))))

(event Input|ActionEvents|InputActionInteract
  (params (Key :type Key%20Structure :default "None"))
  ;[1 1 1] Control
  (:Pressed
    (Utilities|FlowControl|Sequence
      (:then_0
        (for _array_element (Collision|GetOverlappingActors (Variables|Collision|GetCapsuleComponent) 0 :!class /Script/Engine.PrimitiveComponent)
          (bind _asbp_base_interactive (Utilities|Casting|CastToBP_BaseInteractive _array_element))
          (Default|Interact _asbp_base_interactive 0.0))))))

(event Input|AxisEvents|InputAxisForward
  (params (AxisValue :type Float%20%28single-precision%29))
  ;[1 1 1] Control
  (Pawn|Input|AddMovementInput (Transformation|GetActorForwardVector self) AxisValue false))

(event Input|AxisEvents|InputAxisRight
  (params (AxisValue :type Float%20%28single-precision%29))
  ;[1 1 1] Control
  (Pawn|Input|AddMovementInput (Transformation|GetActorRightVector self) AxisValue false))

(event Input|AxisEvents|InputAxismouseX
  (params (AxisValue :type Float%20%28single-precision%29))
  ;[1 1 1] Control
  (Pawn|Input|AddControllerYawInput AxisValue))

(event Input|AxisEvents|InputAxismouseY
  (params (AxisValue :type Float%20%28single-precision%29))
  ;[1 1 1] Control
  (Pawn|Input|AddControllerPitchInput AxisValue))

(event Input|MouseEvents|MouseWheelDown
  (params (Key :type Key%20Structure :default "None"))
  (:Pressed
    (CallFunction|ChangeSelectedWeapon 1)))

(event Input|KeyboardEvents|A
  (params (Key :type Key%20Structure :default "None"))
  (bind _boxchangeentity (Variables|Default|GetboxChangeEntity))
  (bind _overlappingactors (Collision|GetOverlappingActors _boxchangeentity 0 :!class /Script/Engine.PrimitiveComponent))
  ;[1 1 1] Change Entity
  (:Pressed
    (if (Variables|Variable|GetCanChangeEntity?)
      (bind _asbp_player_controller (Utilities|Casting|CastToBP_PlayerController (Game|GetPlayerController 0)))
      (if (Default|CanChangeEntity _asbp_player_controller)
        (if (Utilities|Array|IsNotEmpty _overlappingactors)
          (bind _asbp_player_controller_2 (Utilities|Casting|CastToBP_PlayerController (Game|GetPlayerController 0)))
          (bind _asbp_controllable_entity (Utilities|Casting|CastToBP_ControllableEntity (Utilities|Array|Get(acopy) _overlappingactors)))
          (if (Variables|BP_ControllableEntity_C|GetisControllable? _asbp_controllable_entity)
            (if (Variables|BP_ControllableEntity_C|GetisKnocked? _asbp_controllable_entity)
              (Default|ChangeEntity _asbp_player_controller_2 _asbp_controllable_entity)
              (CallFunction|OnPossesion _asbp_controllable_entity))))))))

(event Input|MouseEvents|MouseWheelUp
  (params (Key :type Key%20Structure :default "None"))
  (:Pressed
    (CallFunction|ChangeSelectedWeapon)))

(event Input|KeyboardEvents|R
  (params (Key :type Key%20Structure :default "None"))
  ;[1 1 1] Control
  (:Pressed
    (Default|Reload (Utilities|Array|Get(acopy) (Variables|WeaponInventory|GetWeaponInventory) (Variables|WeaponInventory|GetCurrentEquipedWeapon)))))

(fn ConstructionScript)

(fn UpdateWalkSpeed
  (params (Max%20Walk%20Speed :type Float%20%28single-precision%29))
  (Variables|/Script/Engine.CharacterMovementComponent|SetMaxWalkSpeed (Variables|Character|GetCharacterMovement) Max%20Walk%20Speed))

(fn AddWeapontoInventory
  (params (WeaponClass :type BP%20Base%20Weapon%20Class%20Reference))
  (if (< (Utilities|Array|Length (Variables|WeaponInventory|GetWeaponInventory)) (Variables|WeaponInventory|GetinventorySize))
    (bind _returnvalue (AddComponent|AddChildActorComponent true (Math|Transform|MakeTransform "0, 0, 0" "0,90.000000,0.000000" "1.000000,1.000000,1.000000")))
    (ChildActorComponent|SetChildActorClass _returnvalue WeaponClass)
    (Transformation|AttachComponentToComponent _returnvalue (Variables|Default|Getarm) "None" "KeepRelative" "KeepRelative" "KeepRelative" true)
    (bind _asbp_base_weapon (Utilities|Casting|CastToBP_BaseWeapon (Variables|/Script/Engine.ChildActorComponent|GetChildActor _returnvalue)))
    (bind _returnvalue_2 (Utilities|Array|Add (Variables|WeaponInventory|GetWeaponInventory) _asbp_base_weapon))
    (return true _returnvalue_2)
    (else
      (return false 0))))

(fn ChangeSelectedWeapon
  (params (WeaponInventoryIndex :type Integer))
  (Utilities|IsValid (Utilities|Array|Get(acopy) (Variables|WeaponInventory|GetWeaponInventory) WeaponInventoryIndex)
    (:Is%20Valid
      (Rendering|SetVisibility (Variables|/Game/Blueprint/Weapon/BP_BaseWeapon.BP_BaseWeapon_C|Getweapon (Utilities|Array|Get(acopy) (Variables|WeaponInventory|GetWeaponInventory) (Variables|WeaponInventory|GetCurrentEquipedWeapon))) false true)
      (bind _output_get (Variables|WeaponInventory|SetCurrentEquipedWeapon WeaponInventoryIndex))
      (Rendering|SetVisibility (Variables|/Game/Blueprint/Weapon/BP_BaseWeapon.BP_BaseWeapon_C|Getweapon (Utilities|Array|Get(acopy) (Variables|WeaponInventory|GetWeaponInventory) _output_get)) true true))))

(fn AddKnockValueFunc
  (params (Value :type Float%20%28double-precision%29))
  (if (Variables|KnockSystem|GetcanBeKnocked?)
    (if (> (+ Value (Variables|KnockSystem|GetknockValue)) (Variables|KnockSystem|GetknockValueMax))
      (Variables|KnockSystem|SetknockValue (Variables|KnockSystem|GetknockValueMax))
      (bind _output_get (Variables|KnockSystem|SetisKnocked? true))
      (Default|ChangeKnockValue (Variables|Default|GetAIController) _output_get)
      (return)
      (else
        (Variables|KnockSystem|SetknockValue (+ (Variables|KnockSystem|GetknockValue) Value))))))

(fn ControllerIAPossese)