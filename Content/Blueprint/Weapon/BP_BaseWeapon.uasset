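; BP_BaseWeapon is a base weapon actor that fires projectiles from an object pool.
; BeginPlay pre-spawns a batch of inactive projectiles, each owned by the BP_ControllableEntity the weapon is attached to.
; GetProjectiles returns the first inactive one, growing the pool by another batch when none is free.
; ShootEvent moves that projectile and its sphere to the spawn point with the weapon's rotation, then activates it after a tiny delay.
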(event Custom|ShootEvent
  (Utilities|Shoot))

(event EventBeginPlay
  (CallFunction|CreateNewProjectilesinPool 50))

(event Collision|EventActorBeginOverlap
  (params (OtherActor :type Actor%20Object%20Reference)))

(event EventTick
  (params (DeltaSeconds :type Float%20%28single-precision%29)))

(fn ConstructionScript)

(fn GetProjectiles
  (bind _array_element (Utilities|Array|ForEachLoopwithBreak (Variables|Default|GetPool) :!label _label)
    (:LoopBody
      (if (not (Variables|/Game/Blueprint/Projectiles/BP_BaseProjectile.BP_BaseProjectile_C|GetisActive? _array_element))
        (return _array_element)))
    (:Completed
      (CallFunction|CreateNewProjectilesinPool 50)
      (goto _label))))

(fn CreateNewProjectilesinPool
  (params (Amount :type Integer))
  (for _index (range 0 Amount)
    (bind _returnvalue (Game|SpawnActorfromClass (Variables|Default|GetProjectiles) (Math|Transform|MakeTransform "0, 0, 0" "0, 0, 0" "1.000000,1.000000,1.000000") "Undefined" 0 0))
    (bind _asbp_controllable_entity (Utilities|Casting|CastToBP_ControllableEntity (Actor|GetAttachParentActor)))
    (Variables|/Game/Blueprint/Projectiles/BP_BaseProjectile.BP_BaseProjectile_C|SetownedPlayer _returnvalue _asbp_controllable_entity)
    (Default|SetActive _returnvalue false)
    (Utilities|Array|Add (Variables|Default|GetPool) _returnvalue)))