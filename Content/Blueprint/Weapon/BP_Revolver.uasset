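; BP_Revolver is the revolver weapon Blueprint, a thin child that relies on its parent class for weapon behavior.
; On BeginPlay it casts the Weapon mesh's anim instance to ABP_Revolver and hands it a reference to itself, then calls the parent BeginPlay.
; If that cast fails, the parent BeginPlay never runs.
; The construction script only calls the parent, and the Tick and overlap events are disabled placeholders.
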(event EventBeginPlay
  (bind _asabp_revolver (Utilities|Casting|CastToABP_Revolver (Components|SkeletalMesh|GetAnimInstance (Variables|Default|Getweapon))))
  (Variables|/Game/Anim/Revolver/ABP_Revolver.ABP_Revolver_C|SetWeapon _asabp_revolver self)
  (|CallParentFunction))

(event Collision|EventActorBeginOverlap
  (params (OtherActor :type Actor%20Object%20Reference))
  (|CallParentFunction OtherActor) ; This node is disabled and will not be called.\nDrag off pins to build functionality.
)

(event EventTick
  (params (DeltaSeconds :type Float%20%28single-precision%29))
  (|CallParentFunction DeltaSeconds) ; This node is disabled and will not be called.\nDrag off pins to build functionality.
)

(fn ConstructionScript
  (|CallParentFunction))