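; Base projectile actor that is toggled on and off through SetActive rather than destroyed, suggesting reuse.
; BeginPlay loads SData from DT_ProjectilesData using the class name as row name, driving gravity, launch speed, lifetime, bouncing and effects.
; Activation launches the physics sphere forward; hits can restore speed and count bounces toward deactivation.
; Overlaps with instigators of another controller class can spawn effects, or deactivate it and apply knock value and damage to BP_ControllableEntity.
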(event OnComponentBeginOverlap(Sphere)
  (params (OverlappedComponent :type Primitive%20Component%20Object%20Reference) (OtherActor :type Actor%20Object%20Reference) (OtherComp :type Primitive%20Component%20Object%20Reference) (OtherBodyIndex :type Integer) (bFromSweep :type Boolean) (SweepResult :type Hit%20Result%20Structure%20%28by%20ref%29))
  (bind _ownedplayer (Variables|Default|GetownedPlayer))
  (bind _instigator (Variables|/Script/Engine.Actor|GetInstigator OtherActor))
  (bind _s_data (Variables|Default|GetS_Data))
  (bind (_path _initialspeed _gravity_ _bouncelimit _impactspeedreduction_ _canbounce_ _destroyafterxtime_ _timebeforedestroy _destroyonentityhit_ _effectondestroy_ _effectonentityhit_) (Utilities|Struct|BreakS_ProjectilesData _s_data))
  (bind _returnvalue (Pawn|GetController _ownedplayer))
  (bind _returnvalue_2 (Utilities|IsValid _instigator))
  (bind _returnvalue_3 (Pawn|GetController _instigator))
  (bind _returnvalue_4 (Utilities|GetClass _returnvalue))
  (bind _returnvalue_5 (Utilities|GetClass _returnvalue_3))
  (bind _returnvalue_6 (!= _returnvalue_5 _returnvalue_4))
  ;[1 1 1] Overlap
  (Utilities|FlowControl|Sequence
    (:then_0
      (if _effectonentityhit_
        (if _returnvalue_2
          (if _returnvalue_6
            (CallFunction|SpawnEffect)))))
    (:then_1
      (if _destroyonentityhit_
        (if _returnvalue_2
          (if _returnvalue_6
            (CallFunction|DisableProjectile)
            (bind _asbp_controllable_entity (Utilities|Casting|CastToBP_ControllableEntity OtherActor))
            (Default|AddKnockValue _asbp_controllable_entity (Variables|Default|GetKnockValue))
            (Game|Damage|ApplyDamage OtherActor (Variables|Default|GetDamage) 0 0)))))))

(event OnComponentHit(Sphere)
  (params (HitComponent :type Primitive%20Component%20Object%20Reference) (OtherActor :type Actor%20Object%20Reference) (OtherComp :type Primitive%20Component%20Object%20Reference) (NormalImpulse :type Vector :default "0, 0, 0") (Hit :type Hit%20Result%20Structure%20%28by%20ref%29))
  (bind _s_data (Variables|Default|GetS_Data))
  (bind (_path _initialspeed _gravity_ _bouncelimit _impactspeedreduction_ _canbounce_) (Utilities|Struct|BreakS_ProjectilesData _s_data))
  (Utilities|FlowControl|Sequence
    (:then_0
      ;[0.3312 0.4138 1] Impact Speed reduction
      (if (not _impactspeedreduction_)
        (Physics|SetPhysicsLinearVelocity (Variables|Default|GetSphere) (* (Math|Vector|Normalize (Transformation|GetComponentVelocity (Variables|Default|GetSphere))) _initialspeed) false "None")))
    (:then_1
      ;[0.3312 0.4138 1] BounceSystem
      (if _canbounce_
        (bind _output_get (Variables|Physics|SetbounceCurrentAmount (+ (Variables|Physics|GetbounceCurrentAmount) 1)))
        (if (and (> _output_get _bouncelimit) (!= _bouncelimit 0))
          (CallFunction|DisableProjectile))))))

(event Custom|DisableProjectile
  (Utilities|FlowControl|Sequence
    (:then_0
      (if (.effectOnDestroy? (Utilities|Struct|BreakS_ProjectilesData (Variables|Default|GetS_Data)))
        (CallFunction|SpawnEffect)))
    (:then_1
      (CallFunction|SetActive false))))

(event Custom|SpawnEffect
  ;[0.8322 0.4238 1] Effect
  (Game|SpawnActorfromClass (.effectClassOnDestroy (Utilities|Struct|BreakS_ProjectilesData (Variables|Default|GetS_Data))) (Math|Transform|MakeTransform (.location (Transformation|GetWorldTransform (Variables|Default|GetSphere))) "0, 0, 0" "1.000000,1.000000,1.000000") "Undefined" 0 0))

(event Custom|OnEnable
  (bind _s_data (Variables|Default|GetS_Data))
  (bind (_path _initialspeed _gravity_ _bouncelimit _impactspeedreduction_ _canbounce_ _destroyafterxtime_ _timebeforedestroy) (Utilities|Struct|BreakS_ProjectilesData _s_data))
  (Utilities|FlowControl|Sequence
    (:then_0
      (Physics|SetEnableGravity (Variables|Default|GetSphere) (.gravity? (Utilities|Struct|BreakS_ProjectilesData (Variables|Default|GetS_Data)))))
    (:then_1
      ;[0.5328 0.75 0.5606] DestroyAfterTime
      (if _destroyafterxtime_
        (Utilities|FlowControl|Delay _timebeforedestroy)
        (if (Variables|Default|GetisActive?)
          (CallFunction|DisableProjectile))))
    (:then_2
      ;[0.3312 0.4138 1] Add Force
      (Physics|SetPhysicsLinearVelocity (Variables|Default|GetSphere) (* (Math|Vector|GetForwardVector (Transformation|GetActorRotation)) _initialspeed) false "None"))))

(event EventBeginPlay
  (CallFunction|SetVariable))

(fn ConstructionScript)

(fn SetVariable
  (bind _returnvalue (Utilities|GetDataTableRow "/Game/Miscellaneous/DT_ProjectilesData.DT_ProjectilesData" (Utilities|String|StringToName (Utilities|String|Replace (Utilities|GetClassDisplayName (Utilities|GetClass self)) "_C" "" "CaseSensitive")))
    (:then
      (Variables|Default|SetS_Data _returnvalue))))

(fn SetActive
  (params (Bool :type Boolean))
  (bind _returnvalue (!= Bool true))
  (bind _sphere (Variables|Default|GetSphere))
  (Actor|Tick|SetActorTickEnabled Bool)
  (Physics|SetSimulatePhysics _sphere Bool)
  (Variables|Default|SetisActive? Bool)
  (Rendering|SetActorHiddenInGame _returnvalue)
  (Development|SetHiddeninGame _sphere _returnvalue false)
  (Variables|/Script/Engine.PrimitiveComponent|SetbGenerateOverlapEvents (Variables|Default|GetSphere) Bool)
  (if Bool
    (CallFunction|OnEnable)))