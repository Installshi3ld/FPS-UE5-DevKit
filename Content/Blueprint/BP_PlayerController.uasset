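; Player controller that runs the timed entity-possession system and creates the main HUD.
; BeginPlay caches the starting pawn as the main entity and loads timer tuning from DT_PlayerData.
; Helpers add capped charge, check its threshold and possess another entity.
; Tick drains the timer per frame assuming 60 FPS; on expiry, a DoOnce destroys the borrowed pawn and, after a short delay, repossesses the main entity, restoring its weapon visibility.
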(event EventTick
  (params (DeltaSeconds :type Float%20%28single-precision%29))
  (bind _bp_maincontrollableentity (Variables|Default|GetBP_MainControllableEntity))
  ;[1 1 1] Change Entity system
  (if (>= (Variables|Default|GettimerChangeEntity) 0.01)
    (Variables|Default|SettimerChangeEntity (- (Variables|Default|GettimerChangeEntity) (/ (Variables|Default|GetsubTimerChangeEntityPerSecond) 6e+01)))
    (goto _label Reset)
    (else
      (Utilities|FlowControl|DoOnce true :!label _label
        (:Completed
          (if (!= (Variables|Default|GetBP_MainControllableEntity) (Pawn|GetControlledPawn))
            (Utilities|FlowControl|Sequence
              (:then_0
                (Utilities|FlowControl|Delay 0.05)
                (CallFunction|ChangeEntity _bp_maincontrollableentity)
                (Utilities|FlowControl|Sequence
                  (:then_0
                    (bind _asbp_base_weapon (Utilities|Casting|CastToBP_BaseWeapon (Variables|/Script/Engine.ChildActorComponent|GetChildActor (Variables|/Game/Blueprint/BP_ControllableEntity.BP_ControllableEntity_C|GetWeapon _bp_maincontrollableentity))))
                    (Rendering|SetVisibility (Variables|/Game/Blueprint/Weapon/BP_BaseWeapon.BP_BaseWeapon_C|Getweapon _asbp_base_weapon) true false))
                  (:then_1
                    (Variables|/Game/Blueprint/BP_ControllableEntity.BP_ControllableEntity_C|SetisControllingEntity? _bp_maincontrollableentity false))))
              (:then_1
                (Actor|DestroyActor (Pawn|GetControlledPawn))))))))))

(event EventBeginPlay
  (Utilities|FlowControl|Sequence
    (:then_0
      (bind _asbp_controllable_entity (Utilities|Casting|CastToBP_ControllableEntity (Pawn|GetControlledPawn)))
      (Variables|Default|SetBP_MainControllableEntity _asbp_controllable_entity)
      (bind _returnvalue (UserInterface|CreateWidget "/Game/Widget/WBP_MainHUD.WBP_MainHUD_C" self))
      (UserInterface|Viewport|AddtoViewport _returnvalue 0))
    (:then_1
      (bind _returnvalue_2 (Utilities|GetDataTableRow "/Game/DataTable/DT_PlayerData.DT_PlayerData" "Player")
        (:then
          (Variables|Default|SetmaxTimerChangeEntity (.maxTimerChangeEntity (Utilities|Struct|BreakS_Player _returnvalue_2)))
          (Variables|Default|SetpercentageChangeEntity (.percentageChanceEntity (Utilities|Struct|BreakS_Player _returnvalue_2)))
          (Variables|Default|SetsubTimerChangeEntityPerSecond (.subTimerChangeEntityPerSecond (Utilities|Struct|BreakS_Player _returnvalue_2))))))))

(fn ConstructionScript)

(fn CanChangeEntity
  (return (>= (/ (Variables|Default|GettimerChangeEntity) (Variables|Default|GetmaxTimerChangeEntity)) (/ (Variables|Default|GetpercentageChangeEntity) 1e+02))))

(fn AddTimertoChangeEntity
  (params (Amount :type Float%20%28double-precision%29))
  (if (>= (+ (Variables|Default|GettimerChangeEntity) Amount) (Variables|Default|GetmaxTimerChangeEntity))
    (Variables|Default|SettimerChangeEntity (Variables|Default|GetmaxTimerChangeEntity))
    (else
      (Variables|Default|SettimerChangeEntity (+ (Variables|Default|GettimerChangeEntity) Amount)))))

(fn ChangeEntity
  (params (OtherEntity :type BP%20Controllable%20Entity%20Object%20Reference))
  (Utilities|FlowControl|Sequence
    (:then_0
      (Pawn|Possess OtherEntity)
      (Variables|/Script/Engine.PrimitiveComponent|SetbGenerateOverlapEvents (Variables|/Game/Blueprint/BP_ControllableEntity.BP_ControllableEntity_C|GetboxChangeEntity OtherEntity) true))))