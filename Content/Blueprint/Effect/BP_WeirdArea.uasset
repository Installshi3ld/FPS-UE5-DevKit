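; BP_WeirdArea is a short-lived ground effect actor built around a scaled cylinder.
; On BeginPlay it traces downward on Visibility, moves to the hit location and plays the BeginShape timeline to drive the cylinder's scale.
; In parallel, a three-second delay plays EndShape in reverse to rescale the cylinder, then destroys the actor.
; The parent BeginPlay call hangs off BeginShape's Update, so it repeats on every timeline update.
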(event EventBeginPlay
  (bind _returnvalue (Transformation|GetActorLocation))
  (Utilities|FlowControl|Sequence
    (:then_0
      (Utilities|FlowControl|Delay 3.0)
      (bind (_direction _scalez _scalexy) (Timeline|EndShape ReverseFromEnd)
        (:Update
          (Transformation|SetWorldScale3D (Variables|Default|GetCylinder) (Math|Vector|MakeVector _scalexy _scalexy _scalez)))
        (:Finished
          (Actor|DestroyActor))))
    (:then_1
      (bind _outhit (Collision|LineTraceByChannel (- _returnvalue "0,0,20.000000") (- _returnvalue "0,0,5000.000000") "TraceTypeQuery1" false 0 "None"))
      (Transformation|SetActorLocation (.Location (Collision|BreakHitResult _outhit)) false false)
      (bind (_direction_2 _scalez_2 _scalexy_2) (Timeline|BeginShape Play)
        (:Update
          (Transformation|SetWorldScale3D (Variables|Default|GetCylinder) (Math|Vector|MakeVector _scalexy_2 _scalexy_2 _scalez_2))
          (|CallParentFunction))))))

(event Collision|EventActorBeginOverlap
  (params (OtherActor :type Actor%20Object%20Reference))
  (|CallParentFunction OtherActor) ; This node is disabled and will not be called.\nDrag off pins to build functionality.
)

(event EventTick
  (params (DeltaSeconds :type Float%20%28single-precision%29))
  (|CallParentFunction DeltaSeconds) ; This node is disabled and will not be called.\nDrag off pins to build functionality.
)

(fn ConstructionScript
  (|CallParentFunction))