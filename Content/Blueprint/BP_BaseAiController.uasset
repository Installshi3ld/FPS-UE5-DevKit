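; Base AI controller that runs the BT_AI behavior tree when it possesses a pawn.
; AI perception updates feed the blackboard: actors tagged "player" set hasLineOfSight and enemyActor when sensed, and clear both when sensing fails.
; An unconnected leftover graph, which never runs, would register the controller on BP_ControllableEntity and loop random wandering with AIMoveTo and a delay.
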(event OnTargetPerceptionUpdated(AIPerception)
  (params (Actor :type Actor%20Object%20Reference) (Stimulus :type AI%20Stimulus%20Structure))
  (bind _returnvalue (Utilities|Name|MakeLiteralName "enemyActor"))
  (bind _returnvalue_2 (Utilities|Name|MakeLiteralName "hasLineOfSight"))
  (bind _blackboard (Variables|Default|GetBlackboard))
  (for _array_element (Variables|/Script/Engine.Actor|GetTags Actor)
    (if (== _array_element "player")
      (if (.bSuccessfullySensed (Utilities|Struct|BreakAIStimulus Stimulus))
        (AI|Components|Blackboard|SetValueasBool _blackboard _returnvalue_2 true)
        (AI|Components|Blackboard|SetValueasObject _blackboard _returnvalue Actor)
        (else
          (AI|Components|Blackboard|SetValueasBool _blackboard _returnvalue_2 false)
          (AI|Components|Blackboard|SetValueasObject _blackboard _returnvalue 0))))))

(event EventUnPossess
  (params (UnpossessedPawn :type Pawn%20Object%20Reference)))

(event EventPossess
  (params (PossessedPawn :type Pawn%20Object%20Reference))
  (AI|RunBehaviorTree "/Game/Blueprint/IA_Behavior/BT_AI.BT_AI"))

(fn ConstructionScript)